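; Dialogue component that runs a behavior-tree-driven conversation when the player interacts, using a GhostMaleTutorial_AI controller spawned at BeginPlay.
; Interact adds a fade widget, pauses the game, blends to an entry camera and opens DialogWidget with UI-only input.
; The widget is passed through the blackboard to the dialogue tree.
; Its exit event stops the tree, restores game input, then fades and pauses again before switching to the exit camera.
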(event Custom|On%20Exit%20Event
  (bind _dialogwidget (Variables|Default|GetDialogWidget))
  (bind _returnvalue (Widget|GetOwningPlayer _dialogwidget))
  ;[1 1 1] Exit Dialog
  (Input|SetInputModeGameOnly _returnvalue)
  (Variables|/Script/Engine.PlayerController|SetbShowMouseCursor _returnvalue false)
  (AI|Logic|StopLogic (Variables|/Script/AIModule.AIController|GetBrainComponent (Variables|Default|GetAIController)) "Exiting Dialog")
  (Widget|RemovefromParent _dialogwidget)
  (bind _returnvalue_2 (UserInterface|CreateWidget "/Game/Blueprints/Widgets/FadeObject.FadeObject_C"))
  (UserInterface|Viewport|AddtoViewport _returnvalue_2 0)
  (Game|SetGamePaused true)
  (Utilities|FlowControl|Delay 0.1)
  (Game|Player|SetViewTargetwithBlend (Game|GetPlayerController 0) (Variables|Default|GetCameraTargetExit) 0.0 "VTBlend_Linear" 0.0 false))

(event EventBeginPlay
  (bind _returnvalue (Game|SpawnActorfromClass "/Game/Blueprints/NPCs/AI_Control/GhostMaleTutorial_AI.GhostMaleTutorial_AI_C" (Math|Transform|MakeTransform "0, 0, 0" "0, 0, 0" "1,1,1") "Undefined" 0 0))
  (Variables|Default|SetAIController _returnvalue))

(event EventInteract
  (params (PlayerCharacter :type Sweater%20Tank%20Object%20Reference))
  (bind _returnvalue (Pawn|GetController PlayerCharacter))
  (bind _aicontroller (Variables|Default|GetAIController))
  (bind _asplayer_controller (Utilities|Casting|CastToPlayerController _returnvalue))
  ;[1 1 1] Set Camera and Open Widget
  (bind _returnvalue_2 (UserInterface|CreateWidget "/Game/Blueprints/Widgets/FadeObject.FadeObject_C"))
  (UserInterface|Viewport|AddtoViewport _returnvalue_2 0)
  (Game|SetGamePaused true)
  (Utilities|FlowControl|Delay 0.1)
  (Game|Player|SetViewTargetwithBlend (Game|GetPlayerController 0) (Variables|Default|GetCameraTargetEnter) 0.0 "VTBlend_Linear" 0.0 false)
  (bind _returnvalue_3 (UserInterface|CreateWidget "/Game/Blueprints/Dialogues/DialogWidget.DialogWidget_C" _asplayer_controller))
  (bind _output_get (Variables|Default|SetDialogWidget _returnvalue_3))
  (EventDispatchers|AssignOnExit _output_get (delegate Custom|On%20Exit%20Event))
  (UserInterface|Viewport|AddtoViewport _returnvalue_3 0)
  (Input|SetInputModeUIOnly _asplayer_controller _returnvalue_3 "DoNotLock")
  (Variables|/Script/Engine.PlayerController|SetbShowMouseCursor _asplayer_controller true)
  ;[1 1 1] Start Dialog Tree
  (AI|RunBehaviorTree _aicontroller (Variables|Default|GetDialogTree))
  (bind _blackboardcomponent (Class|AIController|UseBlackboard _aicontroller "/Game/Blueprints/Dialogues/Blackboards/DialogBlackboard.DialogBlackboard"))
  (AI|Components|Blackboard|SetValueasObject _blackboardcomponent (Utilities|Name|MakeLiteralName "DialogObject") (Variables|Default|GetDialogWidget)))