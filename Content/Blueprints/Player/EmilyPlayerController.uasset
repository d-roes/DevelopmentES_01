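; EmilyPlayerController is a player controller holding unconnected logic for opening an inventory HUD, with no event triggering it.
; That logic creates the InventoryHUD widget, stores it as PlayerInventory, adds it to the viewport and switches input to UI only.
; A gamepad key check decides cursor visibility: hidden for gamepad, shown otherwise, with both branches duplicating the widget setup.
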(event Input|ActionEvents|InputActionInventory
  (params (Key :type Key%20Structure :default "None")))

(fn ConstructionScript)