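; CameraSplineRail is a trigger actor that hands its CameraRail spline to a SceneCamera, defining the rail that camera uses.
; The assignment happens when the player pawn enters the InfluenceRange box, or on BeginPlay if OnStartTrigger is set.
; Leaving the box does nothing, so the camera keeps the last assigned spline.
; The construction script sizes the box from BoxExtent.
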(event OnComponentBeginOverlap(InfluenceRange)
  (params (OverlappedComponent :type Primitive%20Component%20Object%20Reference) (OtherActor :type Actor%20Object%20Reference) (OtherComp :type Primitive%20Component%20Object%20Reference) (OtherBodyIndex :type Integer) (bFromSweep :type Boolean) (SweepResult :type Hit%20Result%20Structure%20%28by%20ref%29))
  (if (== OtherActor (Game|Player|GetPlayerPawn 0))
    (Variables|/Game/Blueprints/Actors/CameraSpline.CameraSpline_C|SetSpline (Variables|Default|GetSceneCamera) (Variables|Default|GetCameraRail))))

(event OnComponentEndOverlap(InfluenceRange)
  (params (OverlappedComponent :type Primitive%20Component%20Object%20Reference) (OtherActor :type Actor%20Object%20Reference) (OtherComp :type Primitive%20Component%20Object%20Reference) (OtherBodyIndex :type Integer)))

(event EventBeginPlay
  (if (Variables|Default|GetOnStartTrigger?)
    (Variables|/Game/Blueprints/Actors/CameraSpline.CameraSpline_C|SetSpline (Variables|Default|GetSceneCamera) (Variables|Default|GetCameraRail))))

(fn ConstructionScript
  (Components|Box|SetBoxExtent (Variables|Default|GetInfluenceRange) (Variables|Default|GetBoxExtent) true))