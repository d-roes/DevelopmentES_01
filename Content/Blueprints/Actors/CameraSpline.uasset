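; Rail camera actor that takes over player 0's view at BeginPlay and follows the pawn along a spline.
; Each tick it eases toward the spline point closest to the pawn.
; A self-recalling Delay loop, separate from Tick, turns the boom and camera toward the pawn while ActiveTrack is set.
; Startup constrains the aspect ratio to a WIREGameInstance setting, and construction sets the boom length.
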(event Custom|LooksAtPlayer
  (bind _returnvalue (Game|Player|GetPlayerPawn 0))
  (bind _cameraspline (Variables|Default|GetCameraSpline))
  (bind _returnvalue_2 (Transformation|GetActorLocation _returnvalue))
  (bind _returnvalue_3 (Transformation|GetWorldLocation _cameraspline))
  (bind _returnvalue_4 (Math|Rotator|FindLookatRotation _returnvalue_3 _returnvalue_2))
  ;[1 1 1] Camera Rotation
  (if (Variables|Default|GetActiveTrack)
    (Transformation|SetWorldRotation (Variables|Default|GetCameraBoom) _returnvalue_4 false false)
    (Transformation|SetWorldRotation (Variables|Default|GetCameraSpline) _returnvalue_4 false false)
    (Utilities|FlowControl|Delay 0.0005)
    (CallFunction|LooksatPlayer)
    (else
      (Utilities|FlowControl|Delay 0.0005)
      (CallFunction|LooksatPlayer))))

(event Custom|MoveCameraOnRail
  (params (DeltaTime :type Float%20%28single-precision%29))
  ;[1 1 1] Camera Movement
  (Transformation|SetActorLocation (Math|Interpolation|VInterpTo (Transformation|GetActorLocation) (Spline|FindLocationClosesttoWorldLocation (Variables|Default|GetSpline) (Transformation|GetActorLocation (Game|Player|GetPlayerPawn 0)) "World") DeltaTime 1.0) false false))

(event EventBeginPlay
  (bind _returnvalue (Game|GetGameInstance))
  (bind _cameraspline (Variables|Default|GetCameraSpline))
  (bind _aswiregame_instance (Utilities|Casting|CastToWIREGameInstance _returnvalue))
  (Game|Player|SetViewTargetwithBlend (Game|GetPlayerController 0) self 0.0 "VTBlend_Linear" 0.0 false)
  (CallFunction|LooksatPlayer)
  (if (Variables|/Game/Blueprints/GameModes/WIREGameInstance.WIREGameInstance_C|GetAspectRatio? _aswiregame_instance)
    (Class|CameraComponent|SetAspectRatio _cameraspline (Variables|/Game/Blueprints/GameModes/WIREGameInstance.WIREGameInstance_C|GetMinAspectRatio _aswiregame_instance))
    (else
      (Class|CameraComponent|SetAspectRatio _cameraspline (Variables|/Game/Blueprints/GameModes/WIREGameInstance.WIREGameInstance_C|GetMaxAspectRatio _aswiregame_instance))))
  (Class|CameraComponent|SetConstraintAspectRatio _cameraspline true))

(event EventTick
  (params (DeltaSeconds :type Float%20%28single-precision%29))
  (CallFunction|MoveCameraonRail DeltaSeconds))

(fn ConstructionScript
  (Variables|/Script/Engine.SpringArmComponent|SetTargetArmLength (Variables|Default|GetCameraBoom) (Variables|Default|GetSpringArmLength)))